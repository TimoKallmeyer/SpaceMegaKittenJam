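; BP_Food is a glowing pickup that raises the cat's Highscore by 500 when collected.
; The construction script gives its point light a random bright tint, and BeginPlay sets each rotation axis to a random 0–1 degree value.
; When the static mesh begins overlapping a BP_Cat, it adds the points directly to that cat and destroys itself.
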(event `self.ReceiveBeginPlay`
  (`self.K2_SetActorRotation` (`KismetMathLibrary.MakeRotator` (`KismetMathLibrary.RandomFloat`) (`KismetMathLibrary.RandomFloat`) (`KismetMathLibrary.RandomFloat`))))

(event `self.StaticMesh.OnComponentBeginOverlap`
  (params (OverlappedComponent :type "PrimitiveComponent Object Reference") (OtherActor :type "Actor Object Reference") (OtherComp :type "PrimitiveComponent Object Reference") (OtherBodyIndex :type Integer) (bFromSweep :type Boolean) (SweepResult :type "HitResult Structure (by ref)"))
  (bind _asbp_cat (cast `/Game/Blueprints/BP_Cat` OtherActor))
  (set `/Game/Blueprints/BP_Cat.Highscore` (+ (`/Game/Blueprints/BP_Cat.Highscore` _asbp_cat) 500.0) _asbp_cat)
  (`self.K2_DestroyActor`))

(fn `UserConstructionScript`
  (`LightComponent.SetLightColor` (`self.PointLight`) (make `LinearColor` (`KismetMathLibrary.RandomFloatInRange` 0.5 1.0) (`KismetMathLibrary.RandomFloatInRange` 0.5 1.0) (`KismetMathLibrary.RandomFloatInRange` 0.5 1.0) 1.0) true))
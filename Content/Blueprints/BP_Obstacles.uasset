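; BP_Obstacles is a randomized obstacle that plays a meow sound when BP_Cat enters its sphere trigger.
; Its construction script adds a random static mesh from ObstacleMeshes and gives the point light a random bright color.
; The same script keeps the actor's location but randomizes its rotation, including roll, and scales each axis independently between ScaleMin and ScaleMax.
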(event `self.StaticMesh.OnComponentHit`
  (params (HitComponent :type "PrimitiveComponent Object Reference") (OtherActor :type "Actor Object Reference") (OtherComp :type "PrimitiveComponent Object Reference") (NormalImpulse :type "Vector Structure") (Hit :type "HitResult Structure (by ref)")))

(event `self.Sphere.OnComponentBeginOverlap`
  (params (OverlappedComponent :type "PrimitiveComponent Object Reference") (OtherActor :type "Actor Object Reference") (OtherComp :type "PrimitiveComponent Object Reference") (OtherBodyIndex :type Integer) (bFromSweep :type Boolean) (SweepResult :type "HitResult Structure (by ref)"))
  (cast `/Game/Blueprints/BP_Cat` OtherActor)
  (`GameplayStatics.PlaySound2D` "/Game/Sounds/SFX/Meow_effect.Meow_effect" 1.0 1.0 0.0 null null))

(fn `UserConstructionScript`
  (bind _obstaclemeshes (`self.ObstacleMeshes`))
  (bind _returnvalue (`KismetMathLibrary.RandomFloatInRange` (`self.ScaleMin`) (`self.ScaleMax`)))
  (`LightComponent.SetLightColor` (`self.PointLight`) (make `LinearColor` (`KismetMathLibrary.RandomFloatInRange` 0.5 1.0) (`KismetMathLibrary.RandomFloatInRange` 0.5 1.0) (`KismetMathLibrary.RandomFloatInRange` 0.5 1.0) 1.0) true)
  (bind _returnvalue_2 (`AddComponent|NODE_AddStaticMeshComponent-0`))
  (`StaticMeshComponent.SetStaticMesh` _returnvalue_2 (`|GetArrayItem` _obstaclemeshes (`KismetMathLibrary.RandomIntegerInRange` 0 (`KismetArrayLibrary.Array_LastIndex` _obstaclemeshes))))
  (`self.K2_SetActorTransform` (`KismetMathLibrary.MakeTransform` (.location (`self.GetTransform`)) (`KismetMathLibrary.RandomRotator` true) (`KismetMathLibrary.MakeVector` _returnvalue _returnvalue _returnvalue))))
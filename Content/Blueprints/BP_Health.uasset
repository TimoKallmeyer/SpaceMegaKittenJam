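; BP_Health is a health pickup actor that BP_Cat collects by overlapping its static mesh.
; On BeginPlay it sets its rotation from raw RandomFloat values, so each axis varies by under one degree.
; On overlap it adds a score bonus proportional to the cat's speed, increments Health and plays an eating sound.
; It then tells HUD_Cat to update the health display and destroys itself.
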(event `self.ReceiveBeginPlay`
  (`self.K2_SetActorRotation` (`KismetMathLibrary.MakeRotator` (`KismetMathLibrary.RandomFloat`) (`KismetMathLibrary.RandomFloat`) (`KismetMathLibrary.RandomFloat`))))

(event `self.StaticMesh.OnComponentBeginOverlap`
  (params (OverlappedComponent :type "PrimitiveComponent Object Reference") (OtherActor :type "Actor Object Reference") (OtherComp :type "PrimitiveComponent Object Reference") (OtherBodyIndex :type Integer) (bFromSweep :type Boolean) (SweepResult :type "HitResult Structure (by ref)"))
  (bind _asbp_cat (cast `/Game/Blueprints/BP_Cat` OtherActor))
  (set `/Game/Blueprints/BP_Cat.Highscore` (+ (`/Game/Blueprints/BP_Cat.Highscore` _asbp_cat) (* 200 (`KismetMathLibrary.Conv_IntToDouble` (/ (`KismetMathLibrary.Round` (`KismetMathLibrary.VSize` (`self.GetVelocity` _asbp_cat))) 100)))) _asbp_cat)
  (`GameplayStatics.PlaySound2D` "/Game/Sounds/SFX/eat_fishy_Cue.eat_fishy_Cue" 1.0 1.0 0.0 null null)
  (`/Engine/EditorBlueprintResources/StandardMacros.IncrementInt` (`/Game/Blueprints/BP_Cat.Health` _asbp_cat)
    (:`  `
      (`/Game/UI/HUD_Cat.Update Health` (cast `/Game/UI/HUD_Cat` (`PlayerController.GetHUD` (`GameplayStatics.GetPlayerController` 0)) :!pure true))
      (`self.K2_DestroyActor`))))

(fn `UserConstructionScript`)
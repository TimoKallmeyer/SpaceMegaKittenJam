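; BP_Tunnel is a procedurally generated, downward-running tube with collision and a color-shifting glow.
; The construction script adds randomly displaced spline points at even depth steps, then lays spline meshes every SectionLength with length-clamped tangents.
; All segments take a dynamic material from MI_Tube01, whose EmissionTint Tick randomizes through a Delay, roughly every 0.75 seconds.
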(event `self.ReceiveTick`
  (params (DeltaSeconds :type "Float (single-precision)"))
  (`KismetSystemLibrary.Delay` 0.75)
  (`MaterialInstanceDynamic.SetVectorParameterValue` (`self.TubeMat`) "EmissionTint" (make `LinearColor` (`KismetMathLibrary.RandomFloatInRange` 0.0 0.5) (`KismetMathLibrary.RandomFloatInRange` 0.0 0.5) (`KismetMathLibrary.RandomFloatInRange` 0.0 0.5) 1.0)))

(fn `UserConstructionScript`
  (bind _counter (`self.Counter`))
  (bind _displacement (`self.Displacement`))
  (bind _displacement_2 (`self.Displacement`))
  (bind _sectionlength (`self.SectionLength`))
  (bind _sectionlength_2 (`self.SectionLength`))
  (bind _spline1 (`self.Spline1`))
  (bind _spline1_2 (`self.Spline1`))
  (bind _returnvalue (`KismetMaterialLibrary.CreateDynamicMaterialInstance` "/Game/Materials/MI_Tube01.MI_Tube01"))
  (set `self.TubeMat` _returnvalue)
  (`SplineComponent.SetLocationAtSplinePoint` (`self.Spline1`) 0 (0.0 0.0 0.0) "World" true)
  (`SplineComponent.SetLocationAtSplinePoint` (`self.Spline1`) 1 (`KismetMathLibrary.MakeVector` 0.0 0.0 (* (* (/ (`self.SplineLengthInMeter`) (`KismetMathLibrary.Conv_IntToDouble` (`self.NumberOfSections`))) 100.0) -1.0)) "World" true)
  (while (not (== (`self.NumberOfSections`) (`self.Counter`)))
    (`/Engine/EditorBlueprintResources/StandardMacros.IncrementInt` _counter
      (:`  `
        (`SplineComponent.AddSplinePoint` (`self.Spline1`) (`KismetMathLibrary.MakeVector` (`KismetMathLibrary.Conv_IntToDouble` (`KismetMathLibrary.RandomIntegerInRange` (* _displacement_2 -1) _displacement_2)) (`KismetMathLibrary.Conv_IntToDouble` (`KismetMathLibrary.RandomIntegerInRange` (* _displacement -1) _displacement)) (* _counter (* (* (/ (`self.SplineLengthInMeter`) (`KismetMathLibrary.Conv_IntToDouble` (`self.NumberOfSections`))) 100.0) -1.0))) "World" true))))
  (for _index (range (`KismetMathLibrary.FTrunc` (/ (`SplineComponent.GetSplineLength` (`self.Spline1`)) (`self.SectionLength`))))
    (bind _returnvalue_2 (`AddComponent|NODE_AddSplineMeshComponent-1`))
    (`SplineMeshComponent.SetForwardAxis` _returnvalue_2 "Z" true)
    (`PrimitiveComponent.SetCollisionEnabled` _returnvalue_2 "QueryAndPhysics")
    (bind _returnvalue_3 (* _index _sectionlength_2))
    (bind _returnvalue_4 (* (+ _index 1) _sectionlength))
    (`SplineMeshComponent.SetStartAndEnd` _returnvalue_2 (`SplineComponent.GetLocationAtDistanceAlongSpline` _spline1 _returnvalue_3 "Local") (`KismetMathLibrary.ClampVectorSize` (`SplineComponent.GetTangentAtDistanceAlongSpline` _spline1 _returnvalue_3 "Local") 0.0 _sectionlength_2) (`SplineComponent.GetLocationAtDistanceAlongSpline` _spline1_2 _returnvalue_4 "Local") (`KismetMathLibrary.ClampVectorSize` (`SplineComponent.GetTangentAtDistanceAlongSpline` _spline1_2 _returnvalue_4 "Local") 0.0 _sectionlength) true)
    (`PrimitiveComponent.CreateDynamicMaterialInstance` _returnvalue_2 0 (`self.TubeMat`) "None")))
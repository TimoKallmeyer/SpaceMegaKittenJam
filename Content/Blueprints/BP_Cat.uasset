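; BP_Cat is a cat Blueprint moved by physics forces on its capsule from player axis input.
; MoveForward and MoveRight push along the actor's forward and right vectors, scaled by axis value, InputMultiplier and current speed, so force is zero at standstill.
; The construction script overrides capsule mass with the Mass variable, and Tick prints speed for debugging.
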(event `InputAxis|MoveForward` :consume false
  (params (AxisValue :type "Float (single-precision)"))
  (`PrimitiveComponent.AddForce` (`self.CapsuleComponent`) (* (`self.GetActorForwardVector`) (* AxisValue (* (`self.InputMultiplier`) (`KismetMathLibrary.VSize` (`self.GetVelocity`))))) "None" false))

(event `self.ReceiveTick`
  (params (DeltaSeconds :type "Float (single-precision)"))
  (`KismetSystemLibrary.PrintString` (`KismetStringLibrary.Conv_DoubleToString` (`KismetMathLibrary.VSize` (`self.GetVelocity`)))))

(event `InputAxis|MoveRight` :consume false
  (params (AxisValue :type "Float (single-precision)"))
  (`PrimitiveComponent.AddForce` (`self.CapsuleComponent`) (* (`self.GetActorRightVector`) (* AxisValue (* (`self.InputMultiplier`) (`KismetMathLibrary.VSize` (`self.GetVelocity`))))) "None" false))

(fn `UserConstructionScript`
  (`PrimitiveComponent.SetMassOverrideInKg` (`self.CapsuleComponent`) "None" (`self.Mass`) true))
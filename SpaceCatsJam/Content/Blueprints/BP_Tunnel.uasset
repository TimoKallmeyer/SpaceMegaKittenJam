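; BP_Tunnel is a spline-based actor that builds a randomly meandering tunnel from spline mesh segments.
; Its Construction Script randomly offsets spline points after the first in world X and Y, bounded by Displacement, keeping Z.
; It then adds colliding, Z-forward spline meshes for each whole SectionLength along the spline, with tangents clamped to that length.
; BeginPlay only prints the spline length for debugging.
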(event `self.ReceiveBeginPlay`
  (`KismetSystemLibrary.PrintString` (`KismetStringLibrary.Conv_DoubleToString` (`SplineComponent.GetSplineLength` (`self.Spline`))) true true (struct :`G` 0.66 :`B` 1.0 :`A` 1.0) 20.0))

(fn `UserConstructionScript`
  (bind _spline (`self.Spline`))
  (bind _displacement (`self.Displacement`))
  (bind _displacement_2 (`self.Displacement`))
  (bind _sectionlength (`self.SectionLength`))
  (bind _sectionlength_2 (`self.SectionLength`))
  (bind _spline_2 (`self.Spline`))
  (for _index (range 1 (+ (`SplineComponent.GetNumberOfSplinePoints` (`self.Spline`)) 1))
    (bind (_returnvalue_x _returnvalue_y _returnvalue_z) (`KismetMathLibrary.BreakVector` (`SplineComponent.GetLocationAtSplinePoint` (`self.Spline`) _index "World")))
    (`SplineComponent.SetLocationAtSplinePoint` (`self.Spline`) _index (`KismetMathLibrary.MakeVector` (+ _returnvalue_x (`KismetMathLibrary.Conv_IntToDouble` (`KismetMathLibrary.RandomIntegerInRange` (* _displacement_2 -1) _displacement_2))) (+ _returnvalue_y (`KismetMathLibrary.Conv_IntToDouble` (`KismetMathLibrary.RandomIntegerInRange` (* _displacement -1) _displacement))) _returnvalue_z) "World" true))
  (for _index_2 (range (`KismetMathLibrary.FTrunc` (/ (`SplineComponent.GetSplineLength` (`self.Spline`)) (`self.SectionLength`))))
    (bind _returnvalue (`AddComponent|NODE_AddSplineMeshComponent-0`))
    (`SplineMeshComponent.SetForwardAxis` _returnvalue "Z" true)
    (`PrimitiveComponent.SetCollisionEnabled` _returnvalue "QueryAndPhysics")
    (bind _returnvalue_2 (* _index_2 _sectionlength_2))
    (bind _returnvalue_3 (* (+ _index_2 1) _sectionlength))
    (`SplineMeshComponent.SetStartAndEnd` _returnvalue (`SplineComponent.GetLocationAtDistanceAlongSpline` _spline_2 _returnvalue_2 "Local") (`KismetMathLibrary.ClampVectorSize` (`SplineComponent.GetTangentAtDistanceAlongSpline` _spline_2 _returnvalue_2 "Local") 0.0 _sectionlength_2) (`SplineComponent.GetLocationAtDistanceAlongSpline` _spline _returnvalue_3 "Local") (`KismetMathLibrary.ClampVectorSize` (`SplineComponent.GetTangentAtDistanceAlongSpline` _spline _returnvalue_3 "Local") 0.0 _sectionlength) true)))